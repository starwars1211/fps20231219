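; BP_PickUpItem is an ammo pickup that refills the current weapon of the main character that overlaps it, then respawns.
; The overlap is handled only with authority, calling a server event that adds AmountToGive to the weapon's CurrentMaxAmmo, clamped to MaxAmmo.
; That event sets IsHidden, waits RespawnTime, then clears it.
; The IsHidden RepNotify toggles sphere collision and actor visibility, so the pickup disappears and returns.
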(event Custom|Server_OnExplosivePickup
  (params (MainCharacter :type BP%20Main%20Character%20Object%20Reference))
  (bind _currenet_weapon (Variables|/Game/Blueprints/BP_MainCharacter.BP_MainCharacter_C|GetCurrenet%20Weapon MainCharacter))
  ;[1 1 1 1 30] 아이템을 먹게되면 사라지게 되고 리스폰 시간이 되면 나타난다
  (Variables|/Game/Blueprints/BP_Weapon_Master.BP_Weapon_Master_C|SetCurrentMaxAmmo _currenet_weapon (Math|Integer|Clamp(Integer) (+ (Variables|/Game/Blueprints/BP_Weapon_Master.BP_Weapon_Master_C|GetCurrentMaxAmmo _currenet_weapon) (Variables|Default|GetAmountToGive)) 0 (Variables|/Game/Blueprints/BP_Weapon_Master.BP_Weapon_Master_C|GetMaxAmmo _currenet_weapon)))
  (Variables|Default|SetIsHidden? true)
  (Utilities|FlowControl|Delay (Variables|Default|GetRespawnTime))
  (Variables|Default|SetIsHidden? false))

(event EventBeginPlay)

(event Collision|EventActorBeginOverlap
  (params (OtherActor :type Actor%20Object%20Reference))
  (Networking|SwitchHasAuthority
    (:Authority
      (bind _asbp_main_character (Utilities|Casting|CastToBP_MainCharacter OtherActor))
      (CallFunction|ServeronExplosivePickup _asbp_main_character))))

(event EventTick
  (params (DeltaSeconds :type Float%20%28single-precision%29)))

(fn ConstructionScript)

(fn OnRepIsHidden?
  ;[1 1 1 1 25] 아이템 히든이냐 아니냐?
  (if (Variables|Default|GetIsHidden?)
    (Collision|SetCollisionEnabled (Variables|Default|GetSphere) "NoCollision")
    (Rendering|SetActorHiddenInGame true)
    (else
      (Collision|SetCollisionEnabled (Variables|Default|GetSphere) "QueryAndPhysics")
      (Rendering|SetActorHiddenInGame false))))