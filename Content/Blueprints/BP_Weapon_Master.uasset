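; Master weapon Blueprint for networked hitscan shooting, with single and automatic fire and clip ammo.
; Client firing runs a randomly spread camera sphere trace, then re-traces from the muzzle toward that point and sends the result to the server.
; Auto fire repeats through a gate-and-delay macro.
; The server decrements the clip and applies damage, or stops the character firing at zero; reload and FX functions are empty stubs.
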(event Custom|Client_OffWeaponFire
  (Utilities|FlowControl|Sequence
    (:then_0
      (Utilities|AitoFireMode) ; enters at Close
    )))

(event Custom|Client_onWeaponFire
  (switch Utilities|FlowControl|Switch|SwitchonE_FiringMode (Variables|Default|GetFiringMode)
    (:NewEnumerator0
      _)
    (:NewEnumerator1
      (Utilities|AitoFireMode
        (:then_0
          _))))
  (bind (_outhit _hit _seeproject _noseeproject) (CallFunction|SphereTrace))
  (CallFunction|ServerShootInfo _outhit _hit _seeproject _noseeproject))

(event Custom|Server_ShootInfo
  (params (OutHit :type Hit%20Result%20Structure%20%28by%20ref%29) (Hit :type Boolean) (SeeProject :type Vector) (NoSeeProject :type Vector))
  (bind _bpmaincharacter (Variables|Default|GetBPMainCharacter))
  (Variables|Default|SetCurrentAmmInClop (Math|Integer|Clamp(Integer) (- (Variables|Default|GetCurrentAmmInClop) 1) 0 (Variables|Default|GetCurrentMaxAmmo)))
  (if (not (== (Variables|Default|GetCurrentAmmInClop) 0))
    (Game|Damage|ApplyDamage (.HitActor (Collision|BreakHitResult OutHit)) (Variables|Default|GetBase%20Damage) (Game|GetInstigatorController) self)
    (else
      (Utilities|IsValid _bpmaincharacter
        (:Is%20Valid
          (Default|ServerStopWeaponFire _bpmaincharacter))))))

(event EventBeginPlay
  (Networking|SwitchHasAuthority
    (:Authority
      (Variables|Default|SetCurrentMaxAmmo (Variables|Default|GetMaxAmmo))
      (Variables|Default|SetCurrentAmmInClop (Variables|Default|GetMaxAmmoClipSize)))))

(event Collision|EventActorBeginOverlap
  (params (OtherActor :type Actor%20Object%20Reference)))

(event EventTick
  (params (DeltaSeconds :type Float%20%28single-precision%29)))

(fn ConstructionScript)

(fn SphereTrace
  (bind _returnvalue (Game|GetPlayerCameraManager 0))
  (bind _returnvalue_2 (Utilities|Name|MakeLiteralName "Muzzle"))
  (bind _returnvalue_3 (Math|Float|MakeLiteralFloat 2.0))
  (bind _returnvalue_4 (Components|GetOwner))
  (bind _sk_rifle_see (Variables|Default|GetSK_Rifle_See))
  (bind _returnvalue_5 (Camera|GetCameraLocation _returnvalue))
  (bind _returnvalue_6 (Transformation|GetSocketLocation _sk_rifle_see _returnvalue_2))
  (bind _array (Utilities|Array|MakeArray _returnvalue_4))
  (bind (_outhit _returnvalue_7) (Collision|SphereTraceByChannel _returnvalue_5 (+ (+ _returnvalue_5 (* (Math|Vector|GetForwardVector (Camera|GetCameraRotation _returnvalue)) 1e+04)) (* (Math|Random|RandomFloatinRange 0.0 3e+02) (Math|Random|RandomUnitVector))) _returnvalue_3 "TraceTypeQuery1" false _array "ForDuration"))
  (bind (_outhit_2 _returnvalue_8) (Collision|SphereTraceByChannel _returnvalue_6 (Math|Vector|SelectVector (.ImpactPoint (Collision|BreakHitResult _outhit)) (.TraceEnd (Collision|BreakHitResult _outhit)) _returnvalue_7) _returnvalue_3 "TraceTypeQuery1" false _array "ForDuration"))
  (return _outhit_2 _returnvalue_8 _returnvalue_6 (Transformation|GetSocketLocation (Variables|Default|GetSK_Rifle_NoSee) _returnvalue_2)))

(fn ReloadAddAmmo)

(fn FireFx)