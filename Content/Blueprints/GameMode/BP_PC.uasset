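; BP_PC is a player controller that handles respawn requests and text chat.
; Server_Respawn passes the controller to BP_GM's ServerRespawnPlayer.
; Enter focuses the UMGChatting text box, and SendMessage prefixes text with the player's name and relays it to every BP_PC.
; Each controller's client receive event then updates its chat widget, if valid.
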(event Custom|Server_Respawn
  (bind _returnvalue (Game|GetGameMode))
  ;[1 1 1 1 25] 게임모드에 리스폰 플레이어를 실행
  (Utilities|IsValid _returnvalue
    (:Is%20Valid
      (bind _asbp_gm (Utilities|Casting|CastToBP_GM _returnvalue))
      (Default|ServerRespawnPlayer _asbp_gm self))))

(event Custom|Cliernt_ReseiveMessage
  (params (Text :type Text))
  (bind _umg_chatting (Variables|Default|GetUMG_Chatting))
  ;[1 1 1] Comment
  (Utilities|IsValid _umg_chatting
    (:Is%20Valid
      (Default|UpdateChat _umg_chatting Text))))

(event Custom|SendMessage
  (params (Text :type Text))
  ;[1 1 1] Comment
  (bind _outactors (Actor|GetAllActorsOfClass "BP_PC_C"))
  (for _array_element _outactors
    (CallFunction|ClierntReseiveMessage _array_element (Utilities|Text|ToText(String) (Utilities|String|Append (PlayerState|GetPlayerName (Variables|GetPlayerState)) ":" (Utilities|String|ToString(Text) Text))))))

(event EventBeginPlay)

(event EventTick
  (params (DeltaSeconds :type Float%20%28single-precision%29)))

(event Input|KeyboardEvents|Enter
  (params (Key :type Key%20Structure :default "None"))
  (bind _umg_chatting (Variables|Default|GetUMG_Chatting))
  (bind _editabletextbox_133 (Variables|/Game/Blueprints/UMG/UMG_Chatting.UMG_Chatting_C|GetEditableTextBox_133 _umg_chatting))
  ;[1 1 1] Comment
  (:Pressed
    (if (not (Class|Widget|HasKeyboardFocus _editabletextbox_133))
      (Widget|SetFocus _editabletextbox_133))))

(fn ConstructionScript)